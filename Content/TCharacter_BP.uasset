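; TCharacter_BP is a character Blueprint that sets up the main HUD and reports health changes.
; On BeginPlay it creates MainHUD_Widget for player 0, adds it to the viewport and binds to HealthComp's OnHealthChanged.
; The bound event only prints the new health and delta to screen as debug output.
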(event `self.ReceiveBeginPlay`
  (bind _returnvalue (`|CreateWidget` "/Game/UI/MainHUD_Widget.MainHUD_Widget_C" (`GameplayStatics.GetPlayerController` 0)))
  (`UserWidget.AddToViewport` _returnvalue 0)
  (add `THealthComponent.OnHealthChanged` (`self.HealthComp`) (delegate `OnHealthChanged_Event_0`)))

(event `OnHealthChanged_Event_0`
  (params (OwningComponent :type "THealthComponent Object Reference") (NewHealth :type Integer) (ActualDelta :type Integer))
  (`KismetSystemLibrary.PrintString` (`KismetStringLibrary.Concat_StrStr` (`KismetStringLibrary.Concat_StrStr` "New Health: " (`KismetStringLibrary.Conv_IntToString` NewHealth)) (`KismetStringLibrary.Concat_StrStr` "  Delta: " (`KismetStringLibrary.Conv_IntToString` ActualDelta)))))

(fn `UserConstructionScript`)